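; BP_ExplosiveTrap is a trap that explodes when a BP_ThirdPersonCharacter enters its sphere trigger.
; The construction script uses a Settings variable to size the trigger and configure the RadialForce radius and impulse strength.
; On overlap it fires the impulse, spawns a short-lived explosion effect, applies radial damage at the force's location, then destroys itself.
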(event `self.SphereCollider.OnComponentBeginOverlap`
  (params (OverlappedComponent :type "PrimitiveComponent Object Reference") (OtherActor :type "Actor Object Reference") (OtherComp :type "PrimitiveComponent Object Reference") (OtherBodyIndex :type Integer) (bFromSweep :type Boolean) (SweepResult :type "HitResult Structure (by ref)"))
  (bind (_settings_triggerrangeradius _settings_explosiverangeradius _settings_explosiveimpulse _settings_explosivebasedamage) (break `/Game/Traps/ExplosiveTrap/S_ExplosiveTrapSettings` (`self.Settings`)))
  (cast `/Game/Characters/BP_ThirdPersonCharacter` OtherActor)
  (`RadialForceComponent.FireImpulse` (`self.RadialForce`))
  (bind _returnvalue (`|SpawnActorFromClass` "/Game/StarterContent/Blueprints/Blueprint_Effect_Explosion.Blueprint_Effect_Explosion_C" (`SceneComponent.K2_GetComponentToWorld` (`self.RadialForce`)) "Undefined" "OverrideRootScale" null null))
  (`self.SetLifeSpan` _returnvalue 4.0)
  (`GameplayStatics.ApplyRadialDamage` :`BaseDamage` _settings_explosivebasedamage :`Origin` (`SceneComponent.K2_GetComponentLocation` (`self.RadialForce`)) :`DamageRadius` _settings_explosiverangeradius :`DamageCauser` null :`InstigatedByController` null)
  (`self.K2_DestroyActor`))

(fn `UserConstructionScript`
  (bind (_settings_triggerrangeradius _settings_explosiverangeradius _settings_explosiveimpulse) (break `/Game/Traps/ExplosiveTrap/S_ExplosiveTrapSettings` (`self.Settings`)))
  (`SphereComponent.SetSphereRadius` (`self.SphereCollider`) _settings_triggerrangeradius true)
  (set `RadialForceComponent.Radius` _settings_explosiverangeradius (`self.RadialForce`))
  (set `RadialForceComponent.ImpulseStrength` _settings_explosiveimpulse (`self.RadialForce`)))