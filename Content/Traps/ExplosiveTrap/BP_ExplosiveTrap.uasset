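; BP_ExplosiveTrap is a proximity trap that explodes when a BP_ThirdPersonCharacter enters its sphere trigger.
; The explosion fires a radial force impulse, spawns a short-lived explosion effect and applies radial damage at the force component's location.
; The construction script sizes the trigger and configures the force from variables, with blast radius shared by impulse and damage.
; DestroyActor is unwired, so the trap persists and can retrigger.
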(event `self.SphereCollider.OnComponentBeginOverlap`
  (params (OverlappedComponent :type "PrimitiveComponent Object Reference") (OtherActor :type "Actor Object Reference") (OtherComp :type "PrimitiveComponent Object Reference") (OtherBodyIndex :type Integer) (bFromSweep :type Boolean) (SweepResult :type "HitResult Structure (by ref)"))
  (cast `/Game/Characters/BP_ThirdPersonCharacter` OtherActor)
  (`RadialForceComponent.FireImpulse` (`self.RadialForce`))
  (bind _returnvalue (`|SpawnActorFromClass` "/Game/StarterContent/Blueprints/Blueprint_Effect_Explosion.Blueprint_Effect_Explosion_C" (`SceneComponent.K2_GetComponentToWorld` (`self.RadialForce`)) "Undefined" "OverrideRootScale" null null))
  (`self.SetLifeSpan` _returnvalue 2.0)
  (`GameplayStatics.ApplyRadialDamage` :`BaseDamage` (`self.ExplosiveBaseDamage`) :`Origin` (`SceneComponent.K2_GetComponentLocation` (`self.RadialForce`)) :`DamageRadius` (`self.ExplosiveRangeRadius`) :`DamageCauser` null :`InstigatedByController` null))

(fn `UserConstructionScript`
  (`SphereComponent.SetSphereRadius` (`self.SphereCollider`) (`self.TriggerRangeRadius`) true)
  (set `RadialForceComponent.Radius` (`self.ExplosiveRangeRadius`) (`self.RadialForce`))
  (set `RadialForceComponent.ImpulseStrength` (`self.ExplosiveImpulse`) (`self.RadialForce`)))