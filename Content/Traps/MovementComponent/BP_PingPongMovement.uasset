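; BP_PingPongMovement is a trap movement component that moves its owning actor between its starting location and a point set by an offset.
; On BeginPlay it derives a round-trip period from offset length and speed, or destroys itself if the offset is near zero.
; Each tick it feeds the wrapped time phase into a float curve to lerp between both points, setting location without sweep, so the curve shapes the motion.
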(event `self.ReceiveBeginPlay`
  (bind _pointboffset (`self.PointBOffset`))
  (if (`KismetMathLibrary.Vector_IsNearlyZero` (`self.PointBOffset`))
    (`self.K2_DestroyComponent`)
    (else
      (bind _output_get (set `self.PointAWorld` (`Actor.K2_GetActorLocation` (`self.GetOwner`))))
      (set `self.PointBWorld` (+ _output_get _pointboffset))
      (set `self.Pediod` (/ (* (`KismetMathLibrary.VSize` _pointboffset) 2.0) (`self.Speed`)))
      (set `self.StartTime` (`GameplayStatics.GetTimeSeconds`)))))

(event `self.ReceiveTick`
  (params (DeltaSeconds :type "Float (single-precision)"))
  (`Actor.K2_SetActorLocation` (`self.GetOwner`) (`KismetMathLibrary.VLerp` (`self.PointAWorld`) (`self.PointBWorld`) (`CurveFloat.GetFloatValue` (`self.MovementCurve`) (mod (/ (- (`GameplayStatics.GetTimeSeconds`) (`self.StartTime`)) (`self.Pediod`)) 1.0))) false false))