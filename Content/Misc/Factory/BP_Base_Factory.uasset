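; Base factory actor that provides a spawn-next-actor hook, left empty here, for producing the next actor in a chain.
; When its recursive spawn flag is set, BeginPlay spawns that actor, attaches it to the factory and stores it as the simulated actor.
; EndPlay then destroys it, so removal cascades down the chain, a behaviour intended mainly for simulations.
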(event `self.ReceiveBeginPlay`
  ;[1 1 1] Mainly for using in simulations because destroying a factory will destroy every next actor in the chain which may not be the desired behaviour
  (if (`self.ShouldSpawnOnBeginPlayRecursively`)
    (bind _out (`/Game/Misc/Factory/BPI_Factory.Spawn Next Actor`))
    (`self.K2_AttachToActor` _out self "None" "KeepRelative" "KeepRelative" "KeepRelative" true)
    (set `self.SimulatedActor` _out)))

(event `self.ReceiveEndPlay`
  (params (EndPlayReason :type "EEndPlayReason Enum" :default "Destroyed"))
  ;[1 1 1] Mainly for using in simulations because destroying a factory will destroy every next actor in the chain which may not be the desired behaviour
  (if (`self.ShouldSpawnOnBeginPlayRecursively`)
    (`self.K2_DestroyActor` (`self.SimulatedActor`))))

(fn `Spawn Next Actor`
  (returns (Out :type "Actor Object Reference"))
  (return null))

(fn `UserConstructionScript`)