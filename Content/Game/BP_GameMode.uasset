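; Game mode that runs a procedurally generated run of branching tile rooms, restarting the level on death or objective completion.
; It spawns a first room, places the player, then offers two next rooms at random exits, one harder with a health bonus.
; Entering a room destroys the others and spawns the next pair until the final room.
; Difficulty settings come from chained, short-lived factory actors spawned and destroyed on demand.
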(event `self.ReceiveBeginPlay`
  (bind _asbp_game_state (cast `/Game/Game/BP_GameState` (`GameplayStatics.GetGameState`)))
  (bind _output_get (set `self.GameStateRef` _asbp_game_state))
  (bind _output_get_2 (set `/Game/Game/BP_GameState.CurrentRoomLevel` 1 _output_get))
  ;[1 1 1] Spawning Entry Rooms
  (bind _out (`self.GetRoomDifficultySettings` _output_get_2))
  (bind (_start_tile_y _exit_1_tile_y _exit_2_tile_y) (`self.GenerateRoomStartsAndExits` (`.TilesCountY_6_C787468F4CCCF825E430C69ED8B39664` (break `/Game/Room/S_RoomDifficultySettings` _out))))
  (bind _returnvalue (`|SpawnActorFromClass` "/Game/Room/BP_Room.BP_Room_C" (`KismetMathLibrary.MakeTransform` (0.0 0.0 0.0)) "Undefined" "OverrideRootScale" null 400.0 400.0 _start_tile_y _exit_1_tile_y _exit_2_tile_y true false "/Game/StarterContent/Materials/M_Wood_Floor_Walnut_Polished.M_Wood_Floor_Walnut_Polished" "/Game/StarterContent/Materials/M_Wood_Pine.M_Wood_Pine" _out false null)) ; Not using BP_Room_Factory to provide specific parameters e.g. Is First
  (set `/Game/Game/BP_GameState.RoomA` _returnvalue (`self.GameStateRef`))
  (`/Game/Room/BP_Room.OpenExitDoors` _returnvalue)
  (`self.SpawnNextRooms`)
  ;[1 1 1] Place Player
  (bind _returnvalue_2 (`GameplayStatics.GetActorOfClass` "/Game/Characters/BP_ThirdPersonCharacter.BP_ThirdPersonCharacter_C"))
  (`self.K2_SetActorTransform` _returnvalue_2 (`KismetMathLibrary.ComposeTransforms` (`KismetMathLibrary.MakeTransform` (0.0 0.0 90.0)) (`/Game/Room/BP_Room.GetStartTileCenterWorldTransform` _returnvalue)) false true))

(event `Main Character Died`
  (bind _asbp_player_controller (cast `/Game/Game/BP_PlayerController` (`GameplayStatics.GetPlayerController` 0))
    (:`then`
      (`/Game/Game/BP_PlayerController.Main Character Died` _asbp_player_controller))
    (:`CastFailed`
      _))
  (`KismetSystemLibrary.Delay` 2.0)
  (`self.RestartLevel`))

(event `RoomEntered`
  (params (Room :type "/Game/Room/BP_Room Object Reference"))
  (bind _gamestateref (`self.GameStateRef`))
  (bind _gamestateref_2 (`self.GameStateRef`))
  (bind _roomb (`/Game/Game/BP_GameState.RoomB` _gamestateref))
  (set `/Game/Game/BP_GameState.IsLoading` true (`self.GameStateRef`))
  (`KismetSystemLibrary.DelayUntilNextTick`) ; Waiting for the frame after rendering the updated IsLoading
  (`KismetSystemLibrary.DelayUntilNextTick`)
  (`/Game/Room/BP_Room.CloseEntryDoor` Room)
  (`self.K2_DestroyActor` (`/Game/Game/BP_GameState.RoomA` _gamestateref))
  (if (== _roomb Room)
    (`self.K2_DestroyActor` (`/Game/Game/BP_GameState.RoomC` _gamestateref))
    (else
      (`self.K2_DestroyActor` _roomb)))
  (bind _output_get (set `/Game/Game/BP_GameState.RoomA` Room _gamestateref_2))
  (`/Engine/EditorBlueprintResources/StandardMacros.IncrementInt` (`/Game/Game/BP_GameState.CurrentRoomLevel` _gamestateref_2)
    (:`  `
      (if (not (`/Game/Room/BP_Room.IsFinal` _output_get))
        (`/Game/Room/BP_Room.OpenExitDoors` _output_get)
        (`self.SpawnNextRooms`)
        (set `/Game/Game/BP_GameState.IsLoading` false (`self.GameStateRef`))))))

(event `GameObjectiveCompleted`
  (bind _asbp_player_controller (cast `/Game/Game/BP_PlayerController` (`GameplayStatics.GetPlayerController` 0))
    (:`then`
      (`/Game/Game/BP_PlayerController.GameObjectiveCompleted` _asbp_player_controller))
    (:`CastFailed`
      _))
  (`KismetSystemLibrary.Delay` 6.0)
  (`self.RestartLevel`))

(fn `GenerateEntryRoomStartAndExits`
  (params (`Tiles Count Y` :type Integer))
  (returns (`Start Tile Y` :type Integer) (`Exit Tile 1 Y` :type Integer) (`Exit Tile 2 Y` :type Integer))
  (locals (ExitTile2Y :type Integer))
  (return (`KismetMathLibrary.RandomIntegerInRange` 0 (- `Tiles Count Y` 1)) 0 0))

(fn `GenerateRoomStartsAndExits`
  (params (`Tiles Count Y` :type Integer))
  (returns (`Start Tile Y` :type Integer) (`Exit 1 Tile Y` :type Integer) (`Exit 2 Tile Y` :type Integer))
  (bind _returnvalue (- `Tiles Count Y` 1))
  (bind _returnvalue_2 (`KismetMathLibrary.RandomIntegerInRange` 0 (- _returnvalue 1)))
  (return (`KismetMathLibrary.RandomIntegerInRange` 0 _returnvalue) _returnvalue_2 (`KismetMathLibrary.RandomIntegerInRange` (+ _returnvalue_2 1) _returnvalue)))

(fn `GetRoomDifficultySettings`
  (params (Number :type Integer :default 1) (IsIncreasedDifficulty :type Boolean))
  (returns (Out :type "/Game/Room/S_RoomDifficultySettings Structure"))
  (locals (Result :type "/Game/Room/S_RoomDifficultySettings Structure"))
  ;[1 1 1] Magic Factories Chain
  (bind _returnvalue (`|SpawnActorFromClass` "/Game/Room/Factories/BP_Difficulty_Factory.BP_Difficulty_Factory_C" (`KismetMathLibrary.MakeTransform` (0.0 0.0 0.0)) "Undefined" "OverrideRootScale" null Number IsIncreasedDifficulty false null))
  (bind _out (`/Game/Room/Factories/BP_Difficulty_Factory.Spawn` _returnvalue))
  (`self.K2_DestroyActor` _returnvalue)
  (bind _out_2 (`/Game/Room/Factories/BP_RoomDifficultySettings_Factory.Spawn` _out))
  (`self.K2_DestroyActor` _out)
  (bind _output_get (set `local.Result` (`/Game/Room/Factories/BP_Room_Factory.DifficultySettings` _out_2)))
  (`self.K2_DestroyActor` _out_2)
  (return _output_get))

(fn `RestartLevel`
  (bind _returnvalue (`GameplayStatics.GetCurrentLevelName` true))
  (`GameplayStatics.OpenLevel` (`KismetStringLibrary.Conv_StringToName` _returnvalue)))

(fn `SpawnNextRooms`
  (locals (LeftRoomVeryRightY :type Integer) (RightRoomVeryLeftY :type Integer) (IsLeftRoomIncreasedDifficultyOne :type Boolean :default false))
  (bind _gamestateref (`self.GameStateRef`))
  (bind _gamestateref_2 (`self.GameStateRef`))
  (bind _rooma (`/Game/Game/BP_GameState.RoomA` (`self.GameStateRef`)))
  (bind _rooma_2 (`/Game/Game/BP_GameState.RoomA` _gamestateref))
  (bind _rooma_3 (`/Game/Game/BP_GameState.RoomA` _gamestateref_2))
  (bind _returnvalue (+ (`/Game/Game/BP_GameState.CurrentRoomLevel` (`self.GameStateRef`)) 1))
  (bind _exit2tiley (`/Game/Room/BP_Room.Exit2TileY` _rooma))
  (bind _output_get (set `local.LeftRoomVeryRightY` (`KismetMathLibrary.RandomIntegerInRange` (`/Game/Room/BP_Room.Exit1TileY` _rooma) (- _exit2tiley 1))))
  (set `local.RightRoomVeryLeftY` (`KismetMathLibrary.RandomIntegerInRange` (+ _output_get 1) _exit2tiley))
  (bind _output_get_2 (set `local.IsLeftRoomIncreasedDifficultyOne` (`KismetMathLibrary.RandomBool`)))
  (`|ExecutionSequence`
    (:`then_0`
      ;[1 1 1] Room B (Left)
      (bind _out (`self.GetRoomDifficultySettings` _returnvalue _output_get_2))
      (bind (_tilescountx _tilescounty) (break `/Game/Room/S_RoomDifficultySettings` _out))
      (bind (_start_tile_y _exit_1_tile_y _exit_2_tile_y) (`self.GenerateRoomStartsAndExits` _tilescounty))
      (bind _returnvalue_2 (`|SpawnActorFromClass` "/Game/Room/BP_Room.BP_Room_C" (`KismetMathLibrary.ComposeTransforms` (`KismetMathLibrary.MakeTransform` (`KismetMathLibrary.MakeVector` (* (`/Game/Room/BP_Room.TilesSizeX` _rooma_3) (`/Game/Room/BP_Room.TilesCountX` _rooma_3)) (* (`/Game/Room/BP_Room.TilesSizeY` _rooma_3) (- (`local.LeftRoomVeryRightY`) _tilescounty -1)))) (`self.GetTransform` (`/Game/Game/BP_GameState.RoomA` (`self.GameStateRef`)))) "Undefined" "OverrideRootScale" null 400.0 400.0 (- _tilescounty (- (`local.LeftRoomVeryRightY`) (`/Game/Room/BP_Room.Exit1TileY` (`/Game/Game/BP_GameState.RoomA` _gamestateref_2))) 1) _exit_1_tile_y _exit_2_tile_y false (== (+ (`/Game/Game/BP_GameState.CurrentRoomLevel` _gamestateref_2) 1) (`/Game/Game/BP_GameState.RoomsCount` _gamestateref_2)) "/Game/StarterContent/Materials/M_Wood_Floor_Walnut_Polished.M_Wood_Floor_Walnut_Polished" "/Game/StarterContent/Materials/M_Wood_Pine.M_Wood_Pine" _out _output_get_2 null))
      (set `/Game/Game/BP_GameState.RoomB` _returnvalue_2 (`self.GameStateRef`)))
    (:`then_1`
      (bind _returnvalue_3 (not _output_get_2))
      ;[1 1 1] Room C (Right)
      (bind _out_2 (`self.GetRoomDifficultySettings` _returnvalue _returnvalue_3))
      (bind (_start_tile_y_2 _exit_1_tile_y_2 _exit_2_tile_y_2) (`self.GenerateRoomStartsAndExits` (`.TilesCountY_6_C787468F4CCCF825E430C69ED8B39664` (break `/Game/Room/S_RoomDifficultySettings` _out_2))))
      (bind _returnvalue_4 (`|SpawnActorFromClass` "/Game/Room/BP_Room.BP_Room_C" (`KismetMathLibrary.ComposeTransforms` (`KismetMathLibrary.MakeTransform` (`KismetMathLibrary.MakeVector` (* (`/Game/Room/BP_Room.TilesSizeX` _rooma_2) (`/Game/Room/BP_Room.TilesCountX` _rooma_2)) (* (`/Game/Room/BP_Room.TilesSizeY` _rooma_2) (`local.RightRoomVeryLeftY`)))) (`self.GetTransform` (`/Game/Game/BP_GameState.RoomA` (`self.GameStateRef`)))) "Undefined" "OverrideRootScale" null 400.0 400.0 (- (`/Game/Room/BP_Room.Exit2TileY` (`/Game/Game/BP_GameState.RoomA` _gamestateref)) (`local.RightRoomVeryLeftY`)) _exit_1_tile_y_2 _exit_2_tile_y_2 false (== (+ (`/Game/Game/BP_GameState.CurrentRoomLevel` _gamestateref) 1) (`/Game/Game/BP_GameState.RoomsCount` _gamestateref)) "/Game/StarterContent/Materials/M_Wood_Floor_Walnut_Polished.M_Wood_Floor_Walnut_Polished" "/Game/StarterContent/Materials/M_Wood_Pine.M_Wood_Pine" _out_2 _returnvalue_3 null))
      (set `/Game/Game/BP_GameState.RoomC` _returnvalue_4 (`self.GameStateRef`)))))

(fn `UserConstructionScript`)