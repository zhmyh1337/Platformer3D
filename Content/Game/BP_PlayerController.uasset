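; Player controller that manages input mode and the screen fade when the main character dies.
; It sets game-only input at BeginPlay.
; On MainCharacterDied it switches to UI-only input with an unlocked mouse, then after a short delay plays the FadeInBlackness animation through BP_HUD's widget.
; A debug binding on the F key unpossesses the current pawn.
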(event `Key|F`
  (params (Key :type "Key Structure"))
  ;[1 1 1] Debug Nodes
  (:`Pressed`
    (`self.UnPossess`)))

(event `self.ReceiveBeginPlay`
  (`WidgetBlueprintLibrary.SetInputMode_GameOnly` self))

(event `Main Character Died`
  (`WidgetBlueprintLibrary.SetInputMode_UIOnlyEx` self null)
  (bind _asbp_hud (cast `/Game/UI/BP_HUD` (`self.GetHUD`)))
  (`KismetSystemLibrary.Delay` 1.0)
  (`/Game/UI/WBP_HUD.Fade In Blackness` (`/Game/UI/BP_HUD.HUD_WBP` _asbp_hud) "Forward" 1.0))

(fn `UserConstructionScript`)