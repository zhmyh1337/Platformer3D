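; Factory that turns a Difficulty value into randomized room settings and spawns the room factory that receives them.
; Tile counts on X and Y are fixed minimums plus random extras scaled by Difficulty.
; Static explosive trap count is the tile area times a random density, capped by a linear bias-and-weight function of Difficulty.
; SpawnNextActor wraps Spawn, which creates the room factory at the origin and passes along the recursive spawn-on-BeginPlay flag.
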(fn ConstructionScript
  (|CallParentFunction))

(fn GetRoomDifficultySettingsbyDifficulty
  (params (Difficulty :type Float%20%28double-precision%29))
  (bind _output_get (LocalVariables|Set@TilesCountX (+ (Math|Random|RandomInteger (Math|Float|Round Difficulty)) 4)))
  (bind _output_get_2 (LocalVariables|Set@TilesCountY (+ (Math|Random|RandomInteger (Math|Float|Round Difficulty)) 3)))
  (bind _output_get_3 (LocalVariables|SetStaticExplosiveTrapsDensity (Math|Random|RandomFloatinRange 0.0 (|(bias+(weight*diff)) 0.5 1.0 Difficulty))))
  (return (Utilities|Struct|MakeS_RoomDifficultySettings _output_get _output_get_2 (Math|Float|Round (* (* (LocalVariables|Get@TilesCountX) (LocalVariables|Get@TilesCountY)) _output_get_3)))))

(fn Spawn
  (bind _difficultysettings (CallFunction|GetRoomDifficultySettingsbyDifficulty (Variables|Default|GetDifficulty)))
  (bind _returnvalue (Game|SpawnActorfromClass "/Game/Room/Factories/BP_Room_Factory.BP_Room_Factory_C" (Math|Transform|MakeTransform "0, 0, 0") "Undefined" 0 _difficultysettings (Variables|Default|GetShouldSpawnOnBeginPlayRecursively) 0))
  (return _returnvalue))

(fn SpawnNextActor
  (bind _out (CallFunction|Spawn))
  (return _out))