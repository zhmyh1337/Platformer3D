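; BP_Difficulty_Factory is a room factory that turns a number and an increased-difficulty flag into a room difficulty value.
; GetRoomDifficulty returns the number, plus a fixed bonus when the flag is set.
; Spawn passes that value and the recursive-spawn flag to a BP_RoomDifficultySettings_Factory spawned at the world origin.
; SpawnNextActor wraps Spawn, making this one link in a chain of factories.
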(fn `GetRoomDifficulty`
  (params (Number :type Integer :default 1) (IsIncreasedDifficulty :type Boolean))
  (returns (Difficulty :type "Float (double-precision)"))
  (locals (DifficultyIncrease :type "Float (double-precision)"))
  (if IsIncreasedDifficulty
    (set `local.DifficultyIncrease` 2.0)
    (else
      (set `local.DifficultyIncrease` 0.0)))
  (return (+ Number (`local.DifficultyIncrease`))))

(fn `Spawn`
  (returns (Out :type "/Game/Room/Factories/BP_RoomDifficultySettings_Factory Object Reference"))
  (bind _difficulty (`self.GetRoomDifficulty` (`self.Number`) (`self.Is Increased Difficulty`)))
  (bind _returnvalue (`|SpawnActorFromClass` "/Game/Room/Factories/BP_RoomDifficultySettings_Factory.BP_RoomDifficultySettings_Factory_C" (`KismetMathLibrary.MakeTransform` (0.0 0.0 0.0)) "Undefined" "OverrideRootScale" null _difficulty (`self.ShouldSpawnOnBeginPlayRecursively`) null))
  (return _returnvalue))

(fn `Spawn Next Actor`
  (returns (Out :type "Actor Object Reference"))
  (bind _out (`self.Spawn`))
  (return _out))

(fn `UserConstructionScript`
  (`parent.UserConstructionScript`))