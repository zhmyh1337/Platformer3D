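; BP_ActorsGenerator is a component of BP_Room that populates the room with gameplay actors, currently a single explosive trap.
; It caches its owning room on BeginPlay.
; GenerateActors spawns BP_ExplosiveTrap with a hardcoded transform and attaches it using KeepRelative, so that transform becomes a room-relative offset.
; EndPlay destroys every actor directly attached to the room.
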(event `self.ReceiveBeginPlay`
  (bind _asbp_room (cast `/Game/Room/BP_Room` (`self.GetOwner`)))
  (set `self.Room` _asbp_room))

(event `self.ReceiveEndPlay`
  (params (EndPlayReason :type "EEndPlayReason Enum" :default "Destroyed"))
  (for _array_element (`Actor.GetAttachedActors` (`self.Room`) true false)
    (`Actor.K2_DestroyActor` _array_element)))

(event `Generate Actors`
  (bind _returnvalue (`|SpawnActorFromClass` "/Game/Traps/ExplosiveTrap/BP_ExplosiveTrap.BP_ExplosiveTrap_C" (`KismetMathLibrary.MakeTransform` (100.0 1000.0 0.0)) "Undefined" "OverrideRootScale" null 200.0 null))
  (`Actor.K2_AttachToActor` _returnvalue (`self.Room`) "None" "KeepRelative" "KeepRelative" "KeepRelative" true))